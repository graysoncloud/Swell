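; Audio-reactive group actor that flashes a random attached PingPongLight in response to audio onsets.
; BeginPlay caches the attached lights; on each Tick with active onsets in the audio manager, one is triggered.
; The first onset's volume scales the base intensity and opacity, with separate fade rates passed to the light.
; Helper functions spawn and attach lights at spline points, optionally skipping the first, or destroy them.
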(event `self.ReceiveBeginPlay`
  ;[1 1 1] BeginPlay
  (`self.FindAllLights`))

(event `self.ReceiveTick`
  (params (DeltaSeconds :type "Float (single-precision)"))
  (bind (_output_timestamp _output_volume) (break `/Game/Blueprints/OnsetTrigger` (`|GetArrayItem` (`/Game/Blueprints/AudioManager.CurrentOnsetTriggers` (`self.AudioManagerRef`)))))
  (`parent.ReceiveTick` DeltaSeconds)
  (if (> (`KismetArrayLibrary.Array_Length` (`/Game/Blueprints/AudioManager.CurrentOnsetTriggers` (`self.AudioManagerRef`))) 0)
    (`self.TriggerRandomLight` _output_volume)))

(fn `DestroyAllLights`
  (`self.FindAllLights`)
  (for _array_element (`self.PingPongLightArray`)
    (`self.K2_DestroyActor` _array_element)))

(fn `FindAllLights`
  (`KismetArrayLibrary.Array_Clear` (`self.PingPongLightArray`))
  (for (_array_element _array_index) (`self.GetAttachedActors` true)
    (bind _asping_pong_light (cast `/Game/Blueprints/AudioReactors/PingPongLight` _array_element))
    (`KismetArrayLibrary.Array_Set` (`self.PingPongLightArray`) _array_index _asping_pong_light true)))

(fn `GenerateAllSplinePoints`
  (for _index (range (`SplineComponent.GetNumberOfSplinePoints` (`self.Spline`)))
    (bind _returnvalue (`|SpawnActorFromClass` "/Game/Blueprints/AudioReactors/PingPongLight.PingPongLight_C" (`KismetMathLibrary.MakeTransform` (`SplineComponent.GetLocationAtSplinePoint` (`self.Spline`) _index "Local")) "Undefined" "OverrideRootScale" null null))
    (`self.K2_AttachToActor` _returnvalue self "None" "KeepRelative" "KeepRelative" "KeepRelative" true)
    (`KismetArrayLibrary.Array_Set` (`self.PingPongLightArray`) _index _returnvalue true))
  (`self.FindAllLights`))

(fn `GenerateAllSplinePoints(excludingFirst)`
  (for _index (range 1 (`SplineComponent.GetNumberOfSplinePoints` (`self.Spline`)))
    (bind _returnvalue (`|SpawnActorFromClass` "/Game/Blueprints/AudioReactors/PingPongLight.PingPongLight_C" (`KismetMathLibrary.MakeTransform` (`SplineComponent.GetLocationAtSplinePoint` (`self.Spline`) _index "Local")) "Undefined" "OverrideRootScale" null null))
    (`self.K2_AttachToActor` _returnvalue self "None" "KeepRelative" "KeepRelative" "KeepRelative" true)
    (`KismetArrayLibrary.Array_Set` (`self.PingPongLightArray`) _index _returnvalue true)))

(fn `TriggerRandomLight`
  (params (IntensityScalar :type "Float (double-precision)"))
  (`/Game/Blueprints/AudioReactors/PingPongLight.TriggerLight` (`|GetArrayItem` (`self.PingPongLightArray`) (`KismetMathLibrary.RandomInteger` (`KismetArrayLibrary.Array_Length` (`self.PingPongLightArray`)))) (* IntensityScalar (`self.BaseLightIntensity`)) (`self.LightIntensityFadeRate`) (* IntensityScalar (`self.BaseLightOpacity`)) (`self.OpacityFadeRate`)))

(fn `UserConstructionScript`
  (`parent.UserConstructionScript`))
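; AudioReactor is an actor that rotates and scales in response to audio swell values.
; A SwellManager passes itself in at game start, and each Tick reads its swell scalar for the rotate and scale targets.
; Rotation speed follows the scalar up to per-axis maximums, while scale lerps toward it on chosen axes with a minimum clamp.
; HandleOnsetTrigger takes a stem but is empty here.
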(event `self.ReceiveTick`
  (params (DeltaSeconds :type "Float (single-precision)"))
  (bind (_returnvalue_x _returnvalue_y _returnvalue_z) (`KismetMathLibrary.BreakVector` (* (* DeltaSeconds (`/Game/Blueprints/SwellManager.GetSwellScalar` (`self.SwellManagerRef`) (`self.Rotate_Target`))) (`self.Rotate_MaxDegreesPerSec`))))
  (`|ExecutionSequence`
    (:`then_0`
      (if (`self.Rotates`)
        (`self.K2_AddActorLocalRotation` (`KismetMathLibrary.MakeRotator` _returnvalue_x _returnvalue_y _returnvalue_z))))
    (:`then_1`
      (if (`self.Scales`)
        (`self.LerpScale` (`/Game/Blueprints/SwellManager.GetSwellScalar` (`self.SwellManagerRef`) (`self.Scale_Target`)) (`self.Scale_Muliplier`) (`self.Scale_LERPStrength`) (`self.Scale_MinScale`) (`self.Scale_Axes`))))))

(fn `HandleOnsetTrigger`
  (params (Stem :type Name)))

(fn `LerpScale`
  (params (NormalizedTarget :type "Float (double-precision)") (Multiplier :type "Float (double-precision)") (Alpha :type "Float (double-precision)") (Minimum :type "Float (double-precision)") (Axes :type "Set of /Game/Blueprints/AudioReactors/Structures/3D-Axis Enum"))
  (bind _returnvalue (* (`local.Multiplier`) (`local.NormalizedTarget`)))
  (bind _result (`/Game/Blueprints/Function_Libraries/BPFL_LERPMath.ClampedMultiAxisVector3LERP` (`local.Axes`) (/ (`self.GetActorRelativeScale3D`) (`self.Scale_Muliplier`)) (`KismetMathLibrary.MakeVector` _returnvalue _returnvalue _returnvalue) (`self.Scale_Muliplier`) (`local.Alpha`) (`local.Minimum`)))
  (`self.SetActorRelativeScale3D` _result))

(fn `SetSwellManager`
  (params (SwellManager :type "/Game/Blueprints/SwellManager Object Reference"))
  ;[1 1 1] SwellManager runs this function (passing itself as a reference) at the start of the game
  (set `self.SwellManagerRef` SwellManager))

(fn `UserConstructionScript`)
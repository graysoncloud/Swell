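; Test audio-reactor Blueprint that drives a Niagara effect's wind from audio onset triggers.
; An onset trigger spikes a stored float, which Tick eases back toward a baseline by a fixed-alpha Lerp, making the decay frame-rate dependent.
; Each tick writes that float to the Niagara WindStrength variable, giving a short gust per onset.
; The onset handler ignores which stem fired, and a swell-based calculation is left unconnected.
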(event `self.ReceiveTick`
  (params (DeltaSeconds :type "Float (single-precision)"))
  (`parent.ReceiveTick` DeltaSeconds)
  (set `self.Floatlol` (`KismetMathLibrary.Lerp` (`self.Floatlol`) 1.0 0.5))
  (`NiagaraComponent.SetVariableFloat` (`self.Niagara`) "WindStrength" (`self.Floatlol`)))

(fn `HandleOnsetTrigger`
  (params (Stem :type "/Game/Blueprints/Structures/Stem_Name Enum" :default "NewEnumerator39"))
  (`parent.HandleOnsetTrigger` Stem)
  (set `self.Floatlol` 25.0))

(fn `UserConstructionScript`
  (`parent.UserConstructionScript`))
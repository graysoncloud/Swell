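; Audio visualizer actor that displays frequency band strengths as a row of glowing cubes.
; SpawnOnConstruct destroys old cubes, then spawns and attaches evenly spaced GlowCube actors along world Y.
; Each Tick reads band strengths from the audio manager and lerps each cube's Z scale toward a scaled, offset target.
; A tutorial P-key play/pause handler, marked deprecated, remains wired; older in-actor Synesthesia analysis and audio setup are disconnected.
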(event `Key|P`
  (params (Key :type "Key Structure"))
  (bind _audio (`self.Audio`))
  ;[1 0.2917 0.2917] DEPRICATED - FROM TUTORIAL
  ;;[0.5972 1 0.5583] Play / Pause / Resume on "P"
  (:`Pressed`
    (if (`AudioComponent.IsPlaying` (`self.Audio`))
      (bind _isa (`/Engine/EditorBlueprintResources/StandardMacros.FlipFlop`)
        (:`A`
          _)
        (:`B`
          _))
      (`AudioComponent.SetPaused` _audio _isa)
      (else
        (`AudioComponent.Play` _audio 0.0)))))

(event `SpawnOnConstruct`
  (bind _glowcubes (`self.SpawnGlowCubes` (`self.Num Glow Cubes`) (`self.Glow Cube Spacing`)))
  (set `self.Glow Cube Array` _glowcubes))

(event `self.ReceiveBeginPlay`)

(event `self.ReceiveTick`
  (params (DeltaSeconds :type "Float (single-precision)"))
  (bind _audiomanagerref (`self.AudioManagerRef`))
  (`/Engine/EditorBlueprintResources/StandardMacros.IsValid` _audiomanagerref
    (:`Is Valid`
      (`self.Synesthesia Scale Cubes` (`/Game/Blueprints/AudioManager.CurrentFreqBandsStrengths` _audiomanagerref)))))

(event `/Game/Blueprints/Interfaces/AudioReactor.Set Audio Parameters`
  (params (NewParam :type Boolean)))

(event `OnPlaybackChange`
  (params (PlayingSoundWave :type "SoundWave Object Reference") (PlaybackPercent :type "Float (single-precision)"))
  ;[1 0.2917 0.2917] DEPRICATED - FROM TUTORIAL
)

(fn `SpawnGlowCubes`
  (params (NumGlowCubes :type Integer) (GlowCubeSpacing :type "Float (double-precision)"))
  (returns (GlowCubes :type "Array of /Game/Blueprints/AudioReactors/GlowCube Object Reference"))
  (bind (_returnvalue_x _returnvalue_y _returnvalue_z) (`KismetMathLibrary.BreakVector` (`SceneComponent.K2_GetComponentLocation` (`self.Root`))))
  ;[1 1 1] Spawn Glow Cubes
  (for _array_element (`self.Glow Cube Array`)
    (`self.K2_DestroyActor` _array_element))
  (`KismetArrayLibrary.Array_Clear` (`self.Glow Cube Array`))
  (for _index (range 1 (+ NumGlowCubes 1))
    (bind _returnvalue (`|SpawnActorFromClass` "/Game/Blueprints/AudioReactors/GlowCube.GlowCube_C" (`KismetMathLibrary.MakeTransform` (`KismetMathLibrary.MakeVector` _returnvalue_x (+ _returnvalue_y (* _index GlowCubeSpacing)) _returnvalue_z) (struct) (0.1 0.1 0.1)) "Undefined" "OverrideRootScale" null null))
    (`self.K2_AttachToActor` _returnvalue self "None" "KeepWorld" "KeepRelative" "KeepRelative" true)
    (`KismetArrayLibrary.Array_Add` (`self.Glow Cube Array`) _returnvalue))
  (return (`self.Glow Cube Array`)))

(fn `Synesthesia Scale Cubes`
  (params (FreqBandsStrengths :type "Array of Float (double-precision)"))
  (locals (FrequencyBandsStrengths :type "Array of Float (single-precision)"))
  ;[0.5972 1 0.5583] Scale our sound cubes according to frequency strengths
  (for (_array_element _array_index) FreqBandsStrengths
    (bind _cube (`/Game/Blueprints/AudioReactors/GlowCube.Cube` (`|GetArrayItem` (`self.Glow Cube Array`) _array_index)))
    (bind _returnvalue (`SceneComponent.GetRelativeTransform` _cube))
    (`SceneComponent.SetRelativeScale3D` _cube (`KismetMathLibrary.MakeVector` (.x (.scale _returnvalue)) (.y (.scale _returnvalue)) (`KismetMathLibrary.Lerp` (.z (.scale _returnvalue)) (+ (* _array_element (`self.CubeZScalingFactor`)) (`self.CubeZScalingOffset`)) (`self.LERPIntensity`))))))

(fn `UserConstructionScript`)
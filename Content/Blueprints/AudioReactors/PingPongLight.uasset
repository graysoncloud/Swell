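; Audio reactor light actor for ping pong that flashes its Sphere mesh when triggered and fades it out.
; BeginPlay creates dynamic material instances for the sphere's materials.
; TriggerLight sets intensity, opacity (with a small added offset) and their fade rates.
; While lit, Tick lowers both values independently, pushing them with the color to the materials until both reach zero or below.
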(event `self.ReceiveBeginPlay`
  (bind _sphere (`self.Sphere`))
  ;[1 1 1] Begin Play (Set up dynamic materials)
  (for (_array_element _array_index) (`MeshComponent.GetMaterials` _sphere)
    (bind _returnvalue (`PrimitiveComponent.CreateDynamicMaterialInstance` _sphere _array_index _array_element "None"))
    (`KismetArrayLibrary.Array_Set` (`self.DynamicMaterials`) _array_index _returnvalue true))
  (`self.UpdateMaterial`))

(event `self.ReceiveTick`
  (params (DeltaSeconds :type "Float (single-precision)"))
  ;[1 1 1] Event tick (update materials)
  (if (`self.LightOn`)
    (set `self.LightIntensity` (- (`self.LightIntensity`) (* DeltaSeconds (`self.LightIntensityFadeRate`))))
    (set `self.Opacity` (- (`self.Opacity`) (* DeltaSeconds (`self.OpacityFadeRate`))))
    (if (and (<= (`self.Opacity`) 0.0) (<= (`self.LightIntensity`) 0.0))
      (set `self.LightOn` false)
      (else
        (`self.UpdateMaterial`)))))

(event `UpdateMaterial`
  ;[1 1 1] Update dynamic material parameters
  (for _array_element (`self.DynamicMaterials`)
    (`MaterialInstanceDynamic.SetVectorParameterValue` _array_element "Color" (`self.Color`))
    (`MaterialInstanceDynamic.SetScalarParameterValue` _array_element "Intensity" (`self.LightIntensity`))
    (`MaterialInstanceDynamic.SetScalarParameterValue` _array_element "Opacity" (`self.Opacity`))))

(fn `TriggerLight`
  (params (LightIntensity :type "Float (double-precision)") (LightIntensityFadeRate :type "Float (double-precision)") (Opacity :type "Float (double-precision)") (OpacityFadeRate :type "Float (double-precision)"))
  (set `self.LightOn` true)
  (set `self.LightIntensity` LightIntensity)
  (set `self.LightIntensityFadeRate` LightIntensityFadeRate)
  (set `self.Opacity` (+ Opacity 0.15))
  (set `self.OpacityFadeRate` OpacityFadeRate))

(fn `UserConstructionScript`)
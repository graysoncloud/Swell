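; Music manager that plays FMOD tracks and exposes audio analysis data, registering itself with every AudioReactor on BeginPlay.
; An AudioPackages map pairs each track with its FMOD event and pre-baked Audio Synesthesia NRT assets.
; While playing, Tick converts timeline position into seconds to sample frequency bands and loudness, and collects normalized onsets since the last update.
; FMOD beat callbacks store bar, beat and tempo.
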(event `self.ReceiveBeginPlay`
  ;[1 1 1] Debugging; set start music
  (bind _outactors (`GameplayStatics.GetAllActorsOfClass` "/Game/Blueprints/AudioReactors/AudioReactor.AudioReactor_C"))
  (bind _output_get (set `self.AudioReactors` _outactors))
  (for _array_element _output_get
    (`/Game/Blueprints/AudioReactors/AudioReactor.SetAudioManager` _array_element self)))

(event `self.FMODAudio.OnTimelineMarker`
  (params (Name :type String) (Position :type Integer))
  ;[1 1 1] On Marker
  (`KismetSystemLibrary.PrintString` (`KismetStringLibrary.Concat_StrStr` "Reached Marker: " Name)))

(event `self.FMODAudio.OnTimelineBeat`
  (params (Bar :type Integer) (Beat :type Integer) (Position :type Integer) (Tempo :type "Float (single-precision)") (TimeSignatureUpper :type Integer) (TimeSignatureLower :type Integer))
  ;[1 1 1] On Beat
  (set `self.Bar` Bar)
  (set `self.Beat` Beat)
  (set `self.Position` Position)
  (set `self.Tempo` Tempo)
  (`KismetSystemLibrary.PrintString` (`KismetStringLibrary.Conv_IntToString` (`self.Beat`))))

(event `InitializeMusic`
  (params (TrackName :type "/Game/Blueprints/TrackName Enum" :default "NewEnumerator0"))
  ;[1 1 1] Initialize Music (Custom Event)
  (`|ExecutionSequence`
    (:`then_0`
      (set `self.CurrentTrack` TrackName)
      (`FMODAudioComponent.SetEvent` (`self.FMODAudio`) (`.FMODEvent_10_87F15DDC434EB75203DAAB9474021998` (break `/Game/Blueprints/AudioPackage` (`BlueprintMapLibrary.Map_Find` (`self.AudioPackages`) TrackName))))
      (set `self.CurrentTrackLength` (`KismetMathLibrary.Conv_IntToDouble` (`FMODAudioComponent.GetLength` (`self.FMODAudio`))))
      (`FMODAudioComponent.Play` (`self.FMODAudio`))
      (add `FMODAudioComponent.OnTimelineBeat` (`self.FMODAudio`) (delegate `OnTimelineBeat_Event`)))
    (:`then_1`
      (set `self.CurrentTrackLength` (`KismetMathLibrary.Conv_IntToDouble` (`FMODAudioComponent.GetLength` (`self.FMODAudio`)))))))

(event `OnTimelineBeat_Event`
  (params (Bar :type Integer) (Beat :type Integer) (Position :type Integer) (Tempo :type "Float (single-precision)") (TimeSignatureUpper :type Integer) (TimeSignatureLower :type Integer))
  ;[1 1 1] Initialize Music (Custom Event)
)

(event `self.ReceiveTick`
  (params (DeltaSeconds :type "Float (single-precision)"))
  ;[1 1 1] Tick
  (bind _returnvalue (`FMODAudioComponent.IsPlaying` (`self.FMODAudio`)))
  (if _returnvalue
    (`self.UpdateSynesthesia`)))

(fn `Play Pause Resume`
  (`self.InitializeMusic` "NewEnumerator1"))

(fn `UpdateSynesthesia`
  (locals (String :type String))
  (bind (_outonsettimestamps _outonsetstrengths) (`OnsetNRT.GetChannelOnsetsBetweenTimes` (`.OnsetNRT_17_9F39B6CD49FFC4420719FAA7767E53A1` (break `/Game/Blueprints/AudioPackage` (`BlueprintMapLibrary.Map_Find` (`self.AudioPackages`) (`self.CurrentTrack`)))) (`self.CurrentTrackElapsedLastTick`) (`self.CurrentTrackElapsedSeconds`) 0))
  (bind _returnvalue (/ (* (`self.CurrentTrackLength`) (`self.CurrentTrackPosition`)) 1000.0))
  (`|ExecutionSequence`
    (:`then_0`
      ;[1 1 1] Update Position
      (bind _returnvalue_2 (`FMODAudioComponent.GetTimelinePosition` (`self.FMODAudio`)))
      (set `self.CurrentTrackPosition` (/ _returnvalue_2 (`self.CurrentTrackLength`))))
    (:`then_1`
      ;[1 1 1] Update frequency band strengths (constant NRT)
      (set `self.CurrentTrackElapsedLastTick` (`self.CurrentTrackElapsedSeconds`))
      (set `self.CurrentTrackElapsedSeconds` _returnvalue)
      (set `self.CurrentFreqBandsStrengths` (`ConstantQNRT.GetNormalizedChannelConstantQAtTime` (`.ConstantNRT_6_A15742CF41120FEE86330B97F2B8B59B` (break `/Game/Blueprints/AudioPackage` (`BlueprintMapLibrary.Map_Find` (`self.AudioPackages`) (`self.CurrentTrack`)))) _returnvalue 0)))
    (:`then_2`
      ;[1 1 1] Update Volume (loudness NRT)
      (set `self.CurrentVolume` (`LoudnessNRT.GetLoudnessAtTime` (`.LoudnessNRT_14_D08570294E91C7B7C87A64BDFCDE89D4` (break `/Game/Blueprints/AudioPackage` (`BlueprintMapLibrary.Map_Find` (`self.AudioPackages`) (`self.CurrentTrack`)))) (`self.CurrentTrackElapsedSeconds`))))
    (:`then_3`
      ;[1 1 1] Update onset triggers (Onset NRT)
      (`KismetArrayLibrary.Array_Clear` (`self.CurrentOnsetTriggers`))
      (for (_array_element _array_index) _outonsettimestamps
        (`KismetArrayLibrary.Array_Set` (`self.CurrentOnsetTriggers`) _array_index (make `/Game/Blueprints/OnsetTrigger` _array_element (`KismetMathLibrary.NormalizeToRange` (`|GetArrayItem` _outonsetstrengths _array_index) (`self.OnsetVolumeMin`) (`self.OnsetVolumeMax`))) true)))))

(fn `UserConstructionScript`)
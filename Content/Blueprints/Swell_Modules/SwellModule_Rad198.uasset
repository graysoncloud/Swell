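; SwellModule_Rad198 is a Swell module that derives a custom audio-reactive float for its Swell Manager.
; Initialize defers to the parent class.
; While the parent update succeeds, each update writes "CustomExample" into the manager's custom floats as the kick stem volume scaled by the inverse of the scalarized beat.
; Otherwise it prints that the manager is inactive.
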(fn `Initialize`
  (params (Swell_Manager :type "/Game/Blueprints/SwellManager Object Reference"))
  (`parent.Initialize` Swell_Manager))

(fn `Update`
  (bind _swellmanager (`self.SwellManager`))
  (bind _swellmanageractive (`parent.Update`))
  (if _swellmanageractive
    (`BlueprintMapLibrary.Map_Add` (`/Game/Blueprints/SwellManager.CustomFloats` (`self.SwellManager`)) "CustomExample" (* (`/Game/Blueprints/SwellManager.GetSwellScalar` _swellmanager "STEMVOL:Kick") (- 1.0 (`/Game/Blueprints/SwellManager.GetSwellScalar` _swellmanager "CUSTOM:ScalarizedBeat"))))
    (else
      (`KismetSystemLibrary.PrintString` null "Swell Manager is inactive; not updating module"))))
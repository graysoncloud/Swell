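; BPFL_ScalarMath is a Blueprint function library of small, independent float math helpers.
; It provides an unclamped cubic smoothstep, remapping to and from a normalized range with safe division, and rounding to hundredths.
; ScalarizeVolume converts a volume value to a clamped 0–1 scalar through a linear offset, so -110 maps to 0 and -10 to 1.
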(fn `DenormalizeScalar`
  (params (Value :type "Float (double-precision)") (Minimum :type "Float (double-precision)") (Maximum :type "Float (double-precision)"))
  (returns (NormalizedScalar :type "Float (double-precision)"))
  (return (+ (* Value (- Maximum (`local.Minimum`))) (`local.Minimum`))))

(fn `NormalizeScalar`
  (params (Value :type "Float (double-precision)") (Minimum :type "Float (double-precision)") (Maximum :type "Float (double-precision)"))
  (returns (NormalizedScalar :type "Float (double-precision)"))
  (return (`KismetMathLibrary.SafeDivide` (- Value Minimum) (- Maximum (`local.Minimum`)))))

(fn `RoundScalarToHundredths`
  (params (Float :type "Float (double-precision)"))
  (returns (RoundedFloat :type "Float (double-precision)"))
  (return (/ (`KismetMathLibrary.Conv_IntToDouble` (`KismetMathLibrary.Round` (* Float 100.0))) 100.0)))

(fn `ScalarizeVolume`
  (params (Volume :type "Float (double-precision)"))
  (returns (ScalarVolume :type "Float (double-precision)"))
  (return (`KismetMathLibrary.FClamp` (+ (/ Volume 100.0) 1.1))))

(fn `Trinomial Smooth`
  (params (InFloat :type "Float (double-precision)"))
  (returns (OutFloat :type "Float (double-precision)"))
  (return (- (* (`KismetMathLibrary.MultiplyMultiply_FloatFloat` InFloat 2.0) 3.0) (* (`KismetMathLibrary.MultiplyMultiply_FloatFloat` InFloat 3.0) 2.0))))
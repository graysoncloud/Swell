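; Blueprint function library for float array math, mainly resizing an array to a new length.
; TransposeArray selects a method: Average blends step-sized index ranges with end indices clamped to a hard-coded 47, while 1to1Repeating wraps the source by modulo.
; The Hash method is an unconnected stub with an empty loop.
; GetAverageOfFloatArray returns a mean; CreateArrayOfSize, the empty-input fallback, caps its loop bound at 1 and returns no array.
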(fn `ArrayTransposition_1to1_Hash`
  (params (ArrToConvert :type "Array of Float (double-precision)") (NewSize :type Integer))
  (locals (StepSize :type "Float (double-precision)") (CurrentVal :type "Float (double-precision)") (ReturnArray :type "Array of Float (double-precision)"))
  (set `local.StepSize` (/ (`KismetArrayLibrary.Array_Length` ArrToConvert) NewSize))
  (for _ (range (`local.NewSize`))
    _))

(fn `ArrayTransposition_Average`
  (params (ArrToConvert :type "Array of Float (double-precision)") (NewSize :type Integer))
  (returns (NewArray :type "Array of Float (double-precision)"))
  (locals (StepSize :type "Float (double-precision)") (CurrentVal :type "Float (double-precision)") (ReturnArray :type "Array of Float (double-precision)"))
  (set `local.StepSize` (/ (`KismetArrayLibrary.Array_Length` ArrToConvert) NewSize))
  (for _index (range (`local.NewSize`))
    (set `local.CurrentVal` 0.0)
    (bind _returnvalue (`KismetMathLibrary.FFloor` (* _index (`local.StepSize`))))
    (bind _returnvalue_2 (`KismetMathLibrary.Clamp` (`KismetMathLibrary.FCeil` (* (+ _index 1) (`local.StepSize`))) 0 47))
    (for _index_2 (range _returnvalue (+ _returnvalue_2 1))
      (set `local.CurrentVal` (+ (`local.CurrentVal`) (/ (`|GetArrayItem` (`local.ArrToConvert`) _index_2) (- _returnvalue_2 _returnvalue)))))
    (`KismetArrayLibrary.Array_Add` (`local.ReturnArray`) (`local.CurrentVal`)))
  (return (`local.ReturnArray`)))

(fn `ArrayTransposition_Repeat`
  (params (ArrToConvert :type "Array of Float (double-precision)") (NewSize :type Integer))
  (returns (ConvertedArray :type "Array of Float (double-precision)"))
  (locals (ReturnArray :type "Array of Float (double-precision)"))
  (bind _returnvalue (`KismetArrayLibrary.Array_Length` ArrToConvert))
  (if (!= _returnvalue 0)
    (for _index (range (`local.NewSize`))
      (`KismetArrayLibrary.Array_Add` (`local.ReturnArray`) (`|GetArrayItem` (`local.ArrToConvert`) (mod _index _returnvalue))))
    (return (`local.ReturnArray`))
    (else
      (return (`self.CreateArrayOfSize` (`local.NewSize`))))))

(fn `CreateArrayOfSize`
  (params (Size :type Integer))
  (returns (NewArray :type "Array of Float (double-precision)"))
  (locals (ReturnArray :type "Array of Float (double-precision)"))
  (for _ (range (+ (`KismetMathLibrary.Min` Size 1) 1))
    (`KismetArrayLibrary.Array_Add` (`local.ReturnArray`)))
  (return))

(fn `GetAverageOfFloatArray`
  (params (FloatArray :type "Array of Float (double-precision)"))
  (returns (AvgValue :type "Float (double-precision)"))
  (locals (Total :type "Float (double-precision)"))
  (bind _total (`local.Total`))
  (for _array_element FloatArray
    (set `local.Total` (+ _total _array_element)))
  (return (/ _total (`KismetArrayLibrary.Array_Length` FloatArray))))

(fn `TransposeArray`
  (params (Method :type "/Game/Blueprints/AudioReactors/zDepricated/Orchestrators/Structures/ArrayTranspositionMethod Enum" :default "NewEnumerator0") (Array :type "Array of Float (double-precision)") (NewSize :type Integer))
  (returns (TransposedArray :type "Array of Float (double-precision)"))
  (return (select `/Game/Blueprints/AudioReactors/zDepricated/Orchestrators/Structures/ArrayTranspositionMethod` (`local.Method`) :`NewEnumerator0` (`self.ArrayTransposition_Average` (`local.Array`) (`local.NewSize`)) :`NewEnumerator1` (`self.ArrayTransposition_Repeat` (`local.Array`) (`local.NewSize`)))))
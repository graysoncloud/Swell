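; String function library with GetSubstringsBySeparator, which splits a string into an array of up to three parts.
; It cuts at the first and last colon, so any colons between them stay in the middle part.
; The leading part is always added, while the middle and trailing parts are added only if non-empty and not already present.
; The Separator input is unused because the colon is hardcoded.
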(fn `GetSubstringsBySeparator`
  (params (InString :type String) (Separator :type String :default ":"))
  (returns (SeparatedStrings :type "Array of String"))
  (locals (BaseString :type String) (ReturnArray :type "Array of String"))
  (bind _returnvalue (`KismetStringLibrary.FindSubstring` InString ":" false true))
  (bind _returnvalue_2 (`KismetStringLibrary.FindSubstring` InString ":"))
  (bind _returnvalue_3 (`KismetStringLibrary.GetSubstring` (`local.BaseString`) (+ _returnvalue_2 1) (- _returnvalue _returnvalue_2 1)))
  (bind _returnvalue_4 (`KismetStringLibrary.GetSubstring` (`local.BaseString`) (+ _returnvalue 1) (- (`KismetStringLibrary.Len` (`local.BaseString`)) _returnvalue)))
  (set `local.BaseString` InString)
  (`KismetArrayLibrary.Array_Add` (`local.ReturnArray`) (`KismetStringLibrary.GetSubstring` (`local.BaseString`) 0 _returnvalue_2))
  (if (not (`KismetStringLibrary.IsEmpty` _returnvalue_3))
    (`KismetArrayLibrary.Array_AddUnique` (`local.ReturnArray`) _returnvalue_3))
  (if (not (`KismetStringLibrary.IsEmpty` _returnvalue_4))
    (`KismetArrayLibrary.Array_AddUnique` (`local.ReturnArray`) _returnvalue_4))
  (return (`local.ReturnArray`)))
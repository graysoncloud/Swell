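; Blueprint function library of interpolation helpers that lerp floats and vectors within clamped or normalized ranges.
; ClampedLERP clamps a float lerp and drives the per-component vector variants for all axes, one enum-selected axis or a set of axes.
; The single-axis variant leaves other axes unchanged, while the multi-axis variant scales excluded axes by a multiplier.
; RangeLERP blends a normalized value toward an optionally inverted target, then maps it back to the range.
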(fn `ClampedLERP`
  (params (A_Val :type "Float (double-precision)") (B_Val :type "Float (double-precision)") (LERPStrength :type "Float (double-precision)") (MinClamp :type "Float (double-precision)") (MaxClamp :type "Float (double-precision)" :default 1000000.0))
  (returns (Result :type "Float (double-precision)"))
  (return (`KismetMathLibrary.FClamp` (`KismetMathLibrary.Lerp` A_Val B_Val LERPStrength) MinClamp MaxClamp)))

(fn `ClampedMultiAxisVector3LERP`
  (params (IncludedAxes :type "Set of /Game/Blueprints/Structures/3D-Axis Enum") (A_Val :type "Vector Structure") (B_Val :type "Vector Structure") (Multiplier :type "Float (double-precision)") (LERPStrength :type "Float (double-precision)") (MinClamp :type "Float (double-precision)") (MaxClamp :type "Float (double-precision)" :default 1000000.0))
  (returns (Result :type "Vector Structure"))
  (bind (_returnvalue_x _returnvalue_y _returnvalue_z) (`KismetMathLibrary.BreakVector` (* (`local.A_Val`) (`local.Multiplier`))))
  (bind _result (`self.ClampedLERP` A_Val_X B_Val_X LERPStrength MinClamp MaxClamp))
  (bind _result_2 (`self.ClampedLERP` A_Val_Y B_Val_Y LERPStrength MinClamp MaxClamp))
  (bind _result_3 (`self.ClampedLERP` A_Val_Z B_Val_Z LERPStrength MinClamp MaxClamp))
  (return (`KismetMathLibrary.MakeVector` (`KismetMathLibrary.SelectFloat` _result _returnvalue_x (`BlueprintSetLibrary.Set_Contains` (`local.IncludedAxes`) "NewEnumerator0")) (`KismetMathLibrary.SelectFloat` _result_2 _returnvalue_y (`BlueprintSetLibrary.Set_Contains` (`local.IncludedAxes`) "NewEnumerator1")) (`KismetMathLibrary.SelectFloat` _result_3 _returnvalue_z (`BlueprintSetLibrary.Set_Contains` (`local.IncludedAxes`) "NewEnumerator2")))))

(fn `ClampedSingleAxisVector3LERP`
  (params (AxisToLERP :type "/Game/Blueprints/Structures/3D-Axis Enum" :default "NewEnumerator1") (A_Val :type "Vector Structure") (B_Val :type "Float (double-precision)") (LERPStrength :type "Float (double-precision)") (MinClamp :type "Float (double-precision)") (MaxClamp :type "Float (double-precision)" :default 1000000.0))
  (returns (Result :type "Vector Structure"))
  (bind (_a_val_x _a_val_y _a_val_z) (`KismetMathLibrary.BreakVector` (`local.A_Val`)))
  (bind _result (`self.ClampedLERP` A_Val_X B_Val LERPStrength MinClamp MaxClamp))
  (bind _result_2 (`self.ClampedLERP` A_Val_Y B_Val LERPStrength MinClamp MaxClamp))
  (bind _result_3 (`self.ClampedLERP` A_Val_Z B_Val LERPStrength MinClamp MaxClamp))
  (return (`KismetMathLibrary.MakeVector` (`KismetMathLibrary.SelectFloat` _result _a_val_x (`|EnumEquality` (`local.AxisToLERP`) "NewEnumerator0")) (`KismetMathLibrary.SelectFloat` _result_2 _a_val_y (`|EnumEquality` (`local.AxisToLERP`) "NewEnumerator1")) (`KismetMathLibrary.SelectFloat` _result_3 _a_val_z (`|EnumEquality` (`local.AxisToLERP`) "NewEnumerator2")))))

(fn `ClampedVector3LERP`
  (params (A_Val :type "Vector Structure") (B_Val :type "Vector Structure") (LERPStrength :type "Float (double-precision)") (MinClamp :type "Float (double-precision)") (MaxClamp :type "Float (double-precision)" :default 1000000.0))
  (returns (Result :type "Vector Structure"))
  (bind _result (`self.ClampedLERP` A_Val_X B_Val_X LERPStrength MinClamp MaxClamp))
  (bind _result_2 (`self.ClampedLERP` A_Val_Y B_Val_Y LERPStrength MinClamp MaxClamp))
  (bind _result_3 (`self.ClampedLERP` A_Val_Z B_Val_Z LERPStrength MinClamp MaxClamp))
  (return (`KismetMathLibrary.MakeVector` _result _result_2 _result_3)))

(fn `RangeLERP`
  (params (Invert :type Boolean) (Minimum :type "Float (double-precision)") (Maximum :type "Float (double-precision)") (RawCurrent :type "Float (double-precision)") (NormalizedTarget :type "Float (double-precision)") (Alpha :type "Float (double-precision)"))
  (returns (NewParam :type "Float (double-precision)"))
  (locals (Range :type "Float (double-precision)") (NormalizedCurrent :type "Float (double-precision)"))
  (return (`/Game/Blueprints/Function_Libraries/BPFL_ScalarMath.DenormalizeScalar` (`KismetMathLibrary.Lerp` (`/Game/Blueprints/Function_Libraries/BPFL_ScalarMath.NormalizeScalar` (`local.RawCurrent`) (`local.Minimum`) (`local.Maximum`)) (`KismetMathLibrary.SelectFloat` (- 1.0 (`local.NormalizedTarget`)) (`local.NormalizedTarget`) (`local.Invert`)) (`local.Alpha`)) (`local.Minimum`) (`local.Maximum`))))
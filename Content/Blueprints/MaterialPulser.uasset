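; MaterialPulser pulses the material of a referenced StaticMeshActor in time with the music.
; BeginPlay creates a dynamic instance of the first material slot and applies its adjusters and color.
; Each Tick, BeatTick adds a pulse on the downbeat of each BarLength cycle from the audio manager, decays all pulses, writes the strongest to PulseParam and refreshes PulseColor.
; An onset-driven OnsetTick exists but is not called here; functions toggle AutoPulse.
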(event `self.ReceiveBeginPlay`
  (`parent.ReceiveBeginPlay`)
  (set `self.StaticMeshComponent` (`self.GetComponentByClass` (`self.StaticMeshActor`) "/Script/Engine.StaticMeshComponent"))
  (bind _returnvalue (`PrimitiveComponent.CreateDynamicMaterialInstance` (`self.StaticMeshComponent`) 0 (`PrimitiveComponent.GetMaterial` (`self.StaticMeshComponent`) 0) "None"))
  (bind _output_get (set `self.DynamicMaterialReference` _returnvalue))
  (`|ExecutionSequence`
    (:`then_0`
      (`MaterialInstanceDynamic.SetScalarParameterValue` _output_get "LERPAdjuster" (`self.LERPAdjuster`)))
    (:`then_1`
      (`MaterialInstanceDynamic.SetScalarParameterValue` _output_get "FadeAdjuster" (`self.FadeAdjuster`)))
    (:`then_2`
      (`MaterialInstanceDynamic.SetScalarParameterValue` _output_get "EmissiveAdjuster" (`self.EmissiveAdjuster`)))
    (:`then_3`
      (`MaterialInstanceDynamic.SetVectorParameterValue` _output_get "PulseColor" (`KismetMathLibrary.Conv_ColorToLinearColor` (`self.Color`))))))

(event `self.ReceiveTick`
  (params (DeltaSeconds :type "Float (single-precision)"))
  (`self.BeatTick` DeltaSeconds)
  (`MaterialInstanceDynamic.SetVectorParameterValue` (`self.DynamicMaterialReference`) "PulseColor" (`KismetMathLibrary.Conv_ColorToLinearColor` (`self.Color`))))

(fn `BeatTick`
  (params (DeltaTime :type "Float (double-precision)"))
  (bind _audiomanagerref (`self.AudioManagerRef`))
  (`|ExecutionSequence`
    (:`then_0`
      (if (and (and (!= (`self.LastBeat`) 1) (== (`/Game/Blueprints/AudioManager.Beat` (`self.AudioManagerRef`)) 1)) (== (mod (+ (`/Game/Blueprints/AudioManager.Bar` _audiomanagerref) -1) (`.BarLength_20_093493644B9C4196F112ACBB5F751176` (break `/Game/Blueprints/AudioPackage` (`BlueprintMapLibrary.Map_Find` (`/Game/Blueprints/AudioManager.AudioPackages` _audiomanagerref) (`/Game/Blueprints/AudioManager.CurrentTrack` _audiomanagerref))))) 0))
        (`KismetArrayLibrary.Array_Add` (`self.PulseStrengths`) 1.0)))
    (:`then_1`
      (if (`KismetArrayLibrary.Array_IsNotEmpty` (`self.PulseStrengths`))
        (set `self.HighestStrength` 0.0)
        (for (_array_element _array_index) (`self.PulseStrengths`)
          (bind _returnvalue (- _array_element (* DeltaTime (`self.PulseRate`))))
          (`KismetArrayLibrary.Array_Set` (`self.PulseStrengths`) _array_index _returnvalue)
          (if (> _returnvalue (`self.HighestStrength`))
            (set `self.HighestStrength` _returnvalue)))))
    (:`then_2`
      (`MaterialInstanceDynamic.SetScalarParameterValue` (`self.DynamicMaterialReference`) "PulseParam" (`self.HighestStrength`)))
    (:`then_3`
      (set `self.LastBeat` (`/Game/Blueprints/AudioManager.Beat` (`self.AudioManagerRef`))))))

(fn `OnsetTick`
  (params (DeltaTime :type "Float (double-precision)"))
  (`|ExecutionSequence`
    (:`then_0`
      (if (`KismetArrayLibrary.Array_IsNotEmpty` (`/Game/Blueprints/AudioManager.CurrentOnsetTriggers` (`self.AudioManagerRef`)))
        (`KismetArrayLibrary.Array_Add` (`self.PulseStrengths`) 1.0)))
    (:`then_1`
      (if (`KismetArrayLibrary.Array_IsNotEmpty` (`self.PulseStrengths`))
        (set `self.HighestStrength` 0.0)
        (for (_ _array_index) (`self.PulseStrengths`)
          (bind _returnvalue (- (`|GetArrayItem` (`self.PulseStrengths`) _array_index) (* DeltaTime 1.0)))
          (`KismetArrayLibrary.Array_Set` (`self.PulseStrengths`) _array_index _returnvalue)
          (if (> _returnvalue (`self.HighestStrength`))
            (set `self.HighestStrength` _returnvalue)))))
    (:`then_2`
      (`MaterialInstanceDynamic.SetScalarParameterValue` (`self.DynamicMaterialReference`) "PulseParam" (* (`self.HighestStrength`) -1.0)))))

(fn `SetMaterialProperties`
  (`MaterialInstanceDynamic.SetScalarParameterValue` (`self.DynamicMaterialReference`) "EmissiveAdjuster" (`self.EmissiveAdjuster`))
  (`MaterialInstanceDynamic.SetScalarParameterValue` (`self.DynamicMaterialReference`) "FadeAdjuster" (`self.FadeAdjuster`))
  (`MaterialInstanceDynamic.SetScalarParameterValue` (`self.DynamicMaterialReference`) "LERPAdjuster" (`self.LERPAdjuster`)))

(fn `ToggleAutoPulseOff`
  (message `AudioParameterControllerInterface.SetBoolParameter` (`self.DynamicMaterialReference`) "AutoPulse" false))

(fn `ToggleAutoPulseOn`
  (message `AudioParameterControllerInterface.SetBoolParameter` (`self.DynamicMaterialReference`) "AutoPulse" true))

(fn `UserConstructionScript`
  (`parent.UserConstructionScript`))